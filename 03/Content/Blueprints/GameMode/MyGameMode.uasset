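; MyGameMode is a game mode that gives each joining player a team and a Champion unit to command.
; On PostLogin, a FlipFlop alternates players between two teams, then a Champion is spawned with its default controller and initialized with that team.
; The player's MyPlayerController stores the Champion as its CommandUnit instead of possessing it.
; On logout, that CommandUnit is destroyed if still valid.
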(event `self.K2_PostLogin`
  (params (NewPlayer :type "PlayerController Object Reference"))
  (`/Engine/EditorBlueprintResources/StandardMacros.FlipFlop`
    (:`A`
      (set `self.Team` "NewEnumerator1"))
    (:`B`
      (set `self.Team` "NewEnumerator2")))
  (bind _returnvalue (`|SpawnActorFromClass` "/Game/Blueprints/Unit/MobileUnit/Champion/Champion.Champion_C" (`KismetMathLibrary.MakeTransform` (0.0 0.0 90.0)) "AdjustIfPossibleButAlwaysSpawn" "OverrideRootScale" null null))
  (`Pawn.SpawnDefaultController` _returnvalue)
  (`/Game/Blueprints/Unit/Unit.Init` _returnvalue (`self.Team`))
  (bind _asmy_player_controller (cast `/Game/Blueprints/PlayerController/MyPlayerController` NewPlayer))
  (set `/Game/Blueprints/PlayerController/MyPlayerController.CommandUnit` _returnvalue _asmy_player_controller))

(event `self.K2_OnLogout`
  (params (ExitingController :type "Controller Object Reference"))
  (bind _asmy_player_controller (cast `/Game/Blueprints/PlayerController/MyPlayerController` ExitingController))
  (bind _commandunit (`/Game/Blueprints/PlayerController/MyPlayerController.CommandUnit` _asmy_player_controller))
  (`/Engine/EditorBlueprintResources/StandardMacros.IsValid` _commandunit
    (:`Is Valid`
      (`self.K2_DestroyActor` _commandunit))))

(fn `UserConstructionScript`)