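; Player controller that lets the player command a single unit by right-clicking in the world, with the mouse cursor shown.
; A right-click, when CommandUnit is valid, line-traces from the deprojected cursor and passes the hit location through the Move event to the unit.
; CommandUnit's RepNotify spawns a MyCamera on the local controller only and sets that unit as its follow target.
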(event `self.ReceiveBeginPlay`
  (set `self.bShowMouseCursor` true))

(event `Move`
  (params (Destination :type "Vector Structure"))
  (`/Game/Blueprints/Unit/Unit.Move` (`self.CommandUnit`) Destination))

(event `InputAction|RightMouseButtonDown`
  (params (Key :type "Key Structure"))
  (bind (_worldlocation _worlddirection) (`self.DeprojectMousePositionToWorld`))
  (:`Pressed`
    (`self.IsCommandUnitValid`
      (:`Is Valid`
        (bind (_outhit _returnvalue) (`KismetSystemLibrary.LineTraceSingle` _worldlocation (+ _worldlocation (* _worlddirection 100000.0)) "TraceTypeQuery3"))
        (if _returnvalue
          (`self.Move` (`.Location` (`GameplayStatics.BreakHitResult` _outhit))))))))

(fn `OnRep_CommandUnit`
  (if (`self.IsLocalPlayerController`)
    (bind _returnvalue (`|SpawnActorFromClass` "/Game/Blueprints/Camera/MyCamera.MyCamera_C" (`KismetMathLibrary.MakeTransform` (0.0 0.0 0.0)) "AlwaysSpawn" "OverrideRootScale" null null))
    (bind _output_get (set `self.MyCamera` _returnvalue))
    (set `/Game/Blueprints/Camera/MyCamera.FollowActor` (`self.CommandUnit`) _output_get)))

(fn `UserConstructionScript`)