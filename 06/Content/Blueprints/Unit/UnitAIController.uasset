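; AI controller for units that carries out Idle, Move, Attack and Attack Move commands.
; SetCommand stops current logic, writes target location or unit to the blackboard (set up on authority) and runs that command's behavior tree.
; It binds to target dispatchers, falling back to Idle or resuming Attack Move when the target dies, is destroyed or hides from its team.
; Helper functions find perceived other-team units by sight or damage, including the nearest living one.
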(event `self.ReceiveBeginPlay`
  (`/Engine/EditorBlueprintResources/ActorMacros.Switch Has Authority`
    (:`Authority`
      (bind _blackboardcomponent (`self.UseBlackboard` "/Game/Blueprints/AI/MyBlackboardData.MyBlackboardData"))
      (set `self.MyBlackboard` _blackboardcomponent))))

(event `SetCommand`
  (params (Command :type "/Game/Blueprints/Enum/Command Enum" :default "NewEnumerator0") (TargetLocation :type "Vector Structure") (TargetUnit :type "/Game/Blueprints/Unit/Unit Object Reference"))
  (bind _braincomponent (`self.BrainComponent`))
  ;[1 1 1] SetCommand
  (`|ExecutionSequence`
    (:`then_0`
      (set `self.Command` Command)
      (`self.ResetTargetUnit`)
      (`/Engine/EditorBlueprintResources/StandardMacros.IsValid` _braincomponent
        (:`Is Valid`
          (`BrainComponent.StopLogic` _braincomponent ""))))
    (:`then_1`
      (switch `/Game/Blueprints/Enum/Command` Command
        (:`NewEnumerator0`
          _)
        (:`NewEnumerator1`
          (`self.SetTargetLocation` TargetLocation))
        (:`NewEnumerator2`
          (`self.SetTargetUnit` TargetUnit))
        (:`NewEnumerator3`
          (`self.SetTargetLocation` TargetLocation)))
      (`self.RunBehaviorTree` (`BlueprintMapLibrary.Map_Find` (`self.BehaviorTrees`) Command)))))

(event `SetTargetLocation`
  (params (TargetLocation :type "Vector Structure"))
  ;[1 1 1] SetTargetLocation
  (bind _output_get (set `self.TargetLocation` TargetLocation))
  (`BlackboardComponent.SetValueAsVector` (`self.MyBlackboard`) (`self.TargetLocationKey`) _output_get))

(event `SetTargetUnit`
  (params (TargetUnit :type "/Game/Blueprints/Unit/Unit Object Reference"))
  ;[1 1 1] SetTargetUnit
  (bind _output_get (set `self.TargetUnit` TargetUnit))
  (`BlackboardComponent.SetValueAsObject` (`self.MyBlackboard`) (`self.TargetUnitKey`) _output_get)
  (`|ExecutionSequence`
    (:`then_0`
      (bind _wrapper (`/Game/Blueprints/Component/EventComponent/GetEventInterface.GetNormalEventDispatcher` (`self.TargetUnit`) "NewEnumerator0"))
      (add `/Game/Blueprints/Component/EventComponent/NormalEventDispatcherWrapper.NormalEventDispatcher` _wrapper (`|CreateDelegate` :!event `AttackCanceldByDeathOrDestroy`)))
    (:`then_1`
      (bind _wrapper_2 (`/Game/Blueprints/Component/EventComponent/GetEventInterface.GetNormalEventDispatcher` (`self.TargetUnit`) "NewEnumerator1"))
      (add `/Game/Blueprints/Component/EventComponent/NormalEventDispatcherWrapper.NormalEventDispatcher` _wrapper_2 (`|CreateDelegate` :!event `AttackCanceldByDeathOrDestroy`)))
    (:`then_2`
      (bind _wrapper_3 (`/Game/Blueprints/Component/EventComponent/GetEventInterface.GetByteEventDispatcher` (`self.TargetUnit`) "NewEnumerator0"))
      (add `/Game/Blueprints/Component/EventComponent/ByteEventDispatcherWrapper.ByteEventDispatcher` _wrapper_3 (`|CreateDelegate` :!event `AttackCanceledByHide`)))))

(event `ResetTargetUnit`
  ;[1 1 1] ResetTargetUnit
  (`/Engine/EditorBlueprintResources/StandardMacros.IsValid` (`self.TargetUnit`)
    (:`Is Valid`
      (`|ExecutionSequence`
        (:`then_0`
          (bind _wrapper (`/Game/Blueprints/Component/EventComponent/GetEventInterface.GetNormalEventDispatcher` (`self.TargetUnit`) "NewEnumerator0"))
          (remove `/Game/Blueprints/Component/EventComponent/NormalEventDispatcherWrapper.NormalEventDispatcher` _wrapper (`|CreateDelegate` :!event `AttackCanceldByDeathOrDestroy`)))
        (:`then_1`
          (bind _wrapper_2 (`/Game/Blueprints/Component/EventComponent/GetEventInterface.GetNormalEventDispatcher` (`self.TargetUnit`) "NewEnumerator1"))
          (remove `/Game/Blueprints/Component/EventComponent/NormalEventDispatcherWrapper.NormalEventDispatcher` _wrapper_2 (`|CreateDelegate` :!event `AttackCanceldByDeathOrDestroy`)))
        (:`then_2`
          (bind _wrapper_3 (`/Game/Blueprints/Component/EventComponent/GetEventInterface.GetByteEventDispatcher` (`self.TargetUnit`) "NewEnumerator0"))
          (remove `/Game/Blueprints/Component/EventComponent/ByteEventDispatcherWrapper.ByteEventDispatcher` _wrapper_3 (`|CreateDelegate` :!event `AttackCanceledByHide`)))
        (:`then_3`
          (set `self.TargetUnit` null)
          (`BlackboardComponent.SetValueAsObject` (`self.MyBlackboard`) (`self.TargetUnitKey`) null))))))

(event `AttackCanceldByDeathOrDestroy`
  (params (Actor :type "Actor Object Reference"))
  ;[1 1 1] AttackCanceldByDeathOrDestroy
  (`self.ResetTargetUnit`)
  (switch `/Game/Blueprints/Enum/Command` (`self.Command`)
    (:`NewEnumerator2`
      (`self.SetCommand` "NewEnumerator0"))
    (:`NewEnumerator3`
      (`self.SetCommand` "NewEnumerator3" (`self.TargetLocation`)))))

(event `AttackCanceledByHide`
  (params (Actor :type "Actor Object Reference") (Byte :type Byte))
  ;[1 1 1] AttackCanceledByHide
  (bind _team (`self.GetOwnerTeam`)
    (:`Get`
      (if (`|EnumEquality` _team (cast `/Game/Blueprints/Enum/Team` Byte))
        (`self.ResetTargetUnit`)
        (switch `/Game/Blueprints/Enum/Command` (`self.Command`)
          (:`NewEnumerator2`
            (`self.SetCommand` "NewEnumerator0"))
          (:`NewEnumerator3`
            (`self.SetCommand` "NewEnumerator3" (`self.TargetLocation`))))))))

(fn `GetNearestAlivePerceivedUnit`
  (params (ContainYellowTeamUnit :type Boolean))
  (returns (Unit :type "/Game/Blueprints/Unit/Unit Object Reference") (Found :type Boolean))
  (locals (LocalUnits :type "Array of /Game/Blueprints/Unit/Unit Object Reference") (NearestUnit :type "/Game/Blueprints/Unit/Unit Object Reference") (OwnerUnit :type "/Game/Blueprints/Unit/Unit Object Reference") (Distance :type "Float (double-precision)"))
  (bind _output (`|GetArrayItem` (`local.LocalUnits`)))
  (if ContainYellowTeamUnit
    (bind _units (`self.GetPerceivedUnits` true))
    (`KismetArrayLibrary.Array_Append` (`local.LocalUnits`) _units)
    (else
      (bind _units_2 (`self.GetPerceivedUnits` true))
      (for _array_element _units_2
        (if (`|EnumInequality` (`/Game/Blueprints/Unit/Unit.Team` _array_element) "NewEnumerator0")
          (`KismetArrayLibrary.Array_Add` (`local.LocalUnits`) _array_element)))))
  (if (> (`KismetArrayLibrary.Array_Length` (`local.LocalUnits`)) 0)
    (bind _asunit (cast `/Game/Blueprints/Unit/Unit` (`self.K2_GetPawn`)))
    (bind _output_get (set `local.OwnerUnit` _asunit))
    (bind _distance (`/Game/Blueprints/Library/MyLibrary.GetUnitDistance` _output_get _output))
    (set `local.NearestUnit` _output)
    (set `local.Distance` _distance)
    (for _array_element_2 (`local.LocalUnits`)
      (bind _distance_2 (`/Game/Blueprints/Library/MyLibrary.GetUnitDistance` _array_element_2 (`local.OwnerUnit`)))
      (if (< _distance_2 (`local.Distance`))
        (set `local.NearestUnit` _array_element_2)
        (set `local.Distance` _distance_2)))
    (return (`local.NearestUnit`) true)
    (else
      (return null false))))

(fn `GetPerceivedUnits`
  (params (Alive :type Boolean))
  (returns (Units :type "Array of /Game/Blueprints/Unit/Unit Object Reference"))
  (locals (LocalUnits :type "Array of /Game/Blueprints/Unit/Unit Object Reference") (LocalAlive :type Boolean) (LocalUnit :type "/Game/Blueprints/Unit/Unit Object Reference"))
  (set `local.LocalAlive` Alive)
  (`|ExecutionSequence`
    (:`then_0`
      (if (`local.LocalAlive`)
        (for _array_element (`AIPerceptionComponent.GetCurrentlyPerceivedActors` (`self.AIPerception`) "/Script/AIModule.AISense_Sight")
          (bind _asunit (cast `/Game/Blueprints/Unit/Unit` _array_element))
          (bind _output_get (set `local.LocalUnit` _asunit))
          (bind _team (`self.GetOwnerTeam`)
            (:`Get`
              (bind _alive (`/Game/Blueprints/Unit/Unit.IsAlive` (`local.LocalUnit`)))
              (if (and _alive (`|EnumInequality` _team (`/Game/Blueprints/Unit/Unit.Team` _output_get)))
                (`KismetArrayLibrary.Array_AddUnique` (`local.LocalUnits`) (`local.LocalUnit`))))))
        (else
          (for _array_element_2 (`AIPerceptionComponent.GetCurrentlyPerceivedActors` (`self.AIPerception`) "/Script/AIModule.AISense_Sight")
            (bind _asunit_2 (cast `/Game/Blueprints/Unit/Unit` _array_element_2))
            (bind _output_get_2 (set `local.LocalUnit` _asunit_2))
            (bind _team_2 (`self.GetOwnerTeam`)
              (:`Get`
                (if (`|EnumInequality` _team_2 (`/Game/Blueprints/Unit/Unit.Team` _output_get_2))
                  (`KismetArrayLibrary.Array_AddUnique` (`local.LocalUnits`) (`local.LocalUnit`)))))))))
    (:`then_1`
      (if (`local.LocalAlive`)
        (for _array_element_3 (`AIPerceptionComponent.GetCurrentlyPerceivedActors` (`self.AIPerception`) "/Script/AIModule.AISense_Damage")
          (bind _asunit_3 (cast `/Game/Blueprints/Unit/Unit` _array_element_3))
          (bind _output_get_3 (set `local.LocalUnit` _asunit_3))
          (bind _team_3 (`self.GetOwnerTeam`)
            (:`Get`
              (bind _alive_2 (`/Game/Blueprints/Unit/Unit.IsAlive` (`local.LocalUnit`)))
              (if (and _alive_2 (`|EnumInequality` _team_3 (`/Game/Blueprints/Unit/Unit.Team` _output_get_3)))
                (`KismetArrayLibrary.Array_AddUnique` (`local.LocalUnits`) (`local.LocalUnit`))))))
        (else
          (for _array_element_4 (`AIPerceptionComponent.GetCurrentlyPerceivedActors` (`self.AIPerception`) "/Script/AIModule.AISense_Damage")
            (bind _asunit_4 (cast `/Game/Blueprints/Unit/Unit` _array_element_4))
            (bind _output_get_4 (set `local.LocalUnit` _asunit_4))
            (bind _team_4 (`self.GetOwnerTeam`)
              (:`Get`
                (if (`|EnumInequality` _team_4 (`/Game/Blueprints/Unit/Unit.Team` _output_get_4))
                  (`KismetArrayLibrary.Array_AddUnique` (`local.LocalUnits`) (`local.LocalUnit`)))))))))
    (:`then_2`
      (return (`local.LocalUnits`)))))

(fn `UserConstructionScript`)