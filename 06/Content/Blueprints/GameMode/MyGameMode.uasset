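; MyGameMode is a game mode that gives each joining player a Champion unit and removes it when they leave.
; PostLogin spawns and initializes a single UnitFactory through a DoOnce, then asks it to spawn a Champion at a fixed point for the new player.
; A FlipFlop alternates successive players between two teams.
; On logout, it destroys the departing MyPlayerController's CommandUnit if valid.
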(event `Init`
  (`/Engine/EditorBlueprintResources/StandardMacros.DoOnce` false
    (:`Completed`
      (bind _returnvalue (`|SpawnActorFromClass` "/Game/Blueprints/GameMode/UnitFactory/UnitFactory.UnitFactory_C" (`KismetMathLibrary.MakeTransform` (0.0 0.0 0.0)) "AlwaysSpawn" "OverrideRootScale" null null))
      (bind _output_get (set `self.UnitFactory` _returnvalue))
      (`/Game/Blueprints/GameMode/UnitFactory/UnitFactory.Init` _output_get))))

(event `self.K2_PostLogin`
  (params (NewPlayer :type "PlayerController Object Reference"))
  (`self.Init`)
  (`/Engine/EditorBlueprintResources/StandardMacros.FlipFlop`
    (:`A`
      (set `self.Team` "NewEnumerator1"))
    (:`B`
      (set `self.Team` "NewEnumerator2")))
  (`/Game/Blueprints/GameMode/UnitFactory/UnitFactory.SpawnUnit` (`self.UnitFactory`) "Champion" (`self.Team`) (`KismetMathLibrary.MakeTransform` (0.0 0.0 90.0)) "AdjustIfPossibleButAlwaysSpawn" NewPlayer))

(event `self.K2_OnLogout`
  (params (ExitingController :type "Controller Object Reference"))
  (bind _asmy_player_controller (cast `/Game/Blueprints/PlayerController/MyPlayerController` ExitingController))
  (bind _commandunit (`/Game/Blueprints/PlayerController/MyPlayerController.CommandUnit` _asmy_player_controller))
  (`/Engine/EditorBlueprintResources/StandardMacros.IsValid` _commandunit
    (:`Is Valid`
      (`self.K2_DestroyActor` _commandunit))))

(fn `UserConstructionScript`)