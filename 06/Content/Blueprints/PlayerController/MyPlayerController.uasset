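; Player controller for mouse-driven command of a single unit, CommandUnit, with a visible cursor.
; Right-click traces under the cursor for a living enemy that passes the team vision check to attack, otherwise sends a ground-location command; middle-click sends another location command type.
; SendCommand forwards commands to the unit's UnitAIController.
; When CommandUnit replicates, the local controller spawns a MyCamera that follows it.
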(event `self.ReceiveBeginPlay`
  (set `self.bShowMouseCursor` true))

(event `InputAction|RightMouseButtonDown`
  (params (Key :type "Key Structure"))
  (bind (_worldlocation _worlddirection) (`self.DeprojectMousePositionToWorld`))
  (bind (_worldlocation_2 _worlddirection_2) (`self.DeprojectMousePositionToWorld`))
  (bind _team (`/Game/Blueprints/Unit/Unit.Team` (`self.CommandUnit`)))
  (:`Pressed`
    (`self.IsCommandUnitValid`
      (:`Is Valid`
        (set `self.AttackUnitFound` false)
        (bind _outhits (`KismetSystemLibrary.LineTraceMulti` _worldlocation_2 (+ _worldlocation_2 (* _worlddirection_2 100000.0)) "TraceTypeQuery4"))
        (for _array_element _outhits
          (bind _asunit (cast `/Game/Blueprints/Unit/Unit` (`.HitActor` (`GameplayStatics.BreakHitResult` _array_element))))
          (bind _alive (`/Game/Blueprints/Unit/Unit.IsAlive` _asunit))
          (bind _vision (`/Game/Blueprints/Unit/Unit.GetVision` _asunit _team))
          (if (and _alive (`|EnumInequality` _vision "NewEnumerator2") (`|EnumInequality` (`/Game/Blueprints/Unit/Unit.Team` _asunit) _team))
            (set `self.AttackUnitFound` true)
            (`self.SendCommand` "NewEnumerator2" (0.0 0.0 0.0) _asunit)
            (break)))
        (if (not (`self.AttackUnitFound`))
          (bind (_outhit _returnvalue) (`KismetSystemLibrary.LineTraceSingle` _worldlocation (+ _worldlocation (* _worlddirection 100000.0)) "TraceTypeQuery3"))
          (if _returnvalue
            (`self.SendCommand` "NewEnumerator1" (`.Location` (`GameplayStatics.BreakHitResult` _outhit)))))))))

(event `InputAction|MiddleMouseButtonDown`
  (params (Key :type "Key Structure"))
  (bind (_worldlocation _worlddirection) (`self.DeprojectMousePositionToWorld`))
  (:`Pressed`
    (bind (_outhit _returnvalue) (`KismetSystemLibrary.LineTraceSingle` _worldlocation (+ _worldlocation (* _worlddirection 100000.0)) "TraceTypeQuery3"))
    (if _returnvalue
      (`self.SendCommand` "NewEnumerator3" (`.Location` (`GameplayStatics.BreakHitResult` _outhit))))))

(event `SendCommand`
  (params (Command :type "/Game/Blueprints/Enum/Command Enum" :default "NewEnumerator0") (TargetLocation :type "Vector Structure") (TargetUnit :type "/Game/Blueprints/Unit/Unit Object Reference"))
  (`self.IsCommandUnitValid`
    (:`Is Valid`
      (bind _asunit_aicontroller (cast `/Game/Blueprints/Unit/UnitAIController` (`AIBlueprintHelperLibrary.GetAIController` (`self.CommandUnit`))))
      (`/Game/Blueprints/Unit/UnitAIController.SetCommand` _asunit_aicontroller Command TargetLocation TargetUnit))))

(fn `OnRep_CommandUnit`
  (if (`self.IsLocalPlayerController`)
    (bind _returnvalue (`|SpawnActorFromClass` "/Game/Blueprints/Camera/MyCamera.MyCamera_C" (`KismetMathLibrary.MakeTransform` (0.0 0.0 0.0)) "AlwaysSpawn" "OverrideRootScale" null null))
    (bind _output_get (set `self.MyCamera` _returnvalue))
    (set `/Game/Blueprints/Camera/MyCamera.FollowActor` (`self.CommandUnit`) _output_get)))

(fn `UserConstructionScript`)