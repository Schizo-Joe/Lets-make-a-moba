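; MyLibrary is a Blueprint library with one helper, GetUnitDistance, that measures the horizontal gap between two units.
; It flattens both actor locations to Z zero and takes the length of their difference.
; It then subtracts both scaled capsule radii, so the result is an edge-to-edge distance that ignores height and goes negative when capsules overlap in plan view.
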(fn `GetUnitDistance`
  (params (Unit0 :type "/Game/Blueprints/Unit/Unit Object Reference") (Unit1 :type "/Game/Blueprints/Unit/Unit Object Reference"))
  (returns (Distance :type "Float (double-precision)"))
  (return (- (`KismetMathLibrary.VSize` (- (`KismetMathLibrary.MakeVector` (.x (`Actor.K2_GetActorLocation` Unit0)) (.y (`Actor.K2_GetActorLocation` Unit0))) (`KismetMathLibrary.MakeVector` (.x (`Actor.K2_GetActorLocation` Unit1)) (.y (`Actor.K2_GetActorLocation` Unit1))))) (+ (`CapsuleComponent.GetScaledCapsuleRadius` (`Character.CapsuleComponent` Unit0)) (`CapsuleComponent.GetScaledCapsuleRadius` (`Character.CapsuleComponent` Unit1))))))