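; Actor component that tracks current HP and MP for an owning Unit and reports whether it is alive.
; Events add a clamped amount to either value, fully restore both, or recover a percentage of each maximum.
; GetMaxHP and GetMaxMP macros cast the owner to Unit and read its parameters, so updates stop when that cast fails.
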(event `AddHP`
  (params (Amount :type "Float (double-precision)"))
  (bind _maxhp (`self.GetMaxHP`)
    (:`Get`
      (set `self.CurHP` (`KismetMathLibrary.FClamp` (+ Amount (`self.CurHP`)) 0.0 _maxhp)))))

(event `AddMP`
  (params (Amount :type "Float (double-precision)"))
  (bind _maxmp (`self.GetMaxMP`)
    (:`Get`
      (set `self.CurMP` (`KismetMathLibrary.FClamp` (+ Amount (`self.CurMP`)) 0.0 _maxmp)))))

(event `FullRecovery`
  (bind _maxhp (`self.GetMaxHP`)
    (:`Get`
      (set `self.CurHP` _maxhp)
      (bind _maxmp (`self.GetMaxMP`)
        (:`Get`
          (set `self.CurMP` _maxmp))))))

(event `PercentRecovery`
  (params (Percent :type "Float (double-precision)"))
  (bind _maxhp (`self.GetMaxHP`)
    (:`Get`
      (`self.AddHP` (* _maxhp Percent))
      (bind _maxmp (`self.GetMaxMP`)
        (:`Get`
          (`self.AddMP` (* _maxmp Percent)))))))

(fn `IsAlive`
  (returns (Alive :type Boolean))
  (return (> (`self.CurHP`) 0.0)))