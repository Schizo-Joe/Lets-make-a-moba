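; Level component for a Unit that tracks experience and level and supplies per-level stat values.
; On BeginPlay it caches the level table referenced by the unit's data table row into a map keyed by level.
; The authority then sets the starting level and fully restores HP/MP, while AddExp triggers recursive level-ups against Exp thresholds.
; GetAddParam returns the current level's value for a requested stat, and GetMulParam is always neutral.
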(event `self.ReceiveBeginPlay`
  (`self.Init`))

(event `Init`
  (bind _returnvalue (`Actor.GetComponentByClass` (`self.GetOwner`) "/Game/Blueprints/Component/HPMPComponent.HPMPComponent_C"))
  (`BlueprintMapLibrary.Map_Clear` (`self.UnitLevelData`))
  (bind _asunit (cast `/Game/Blueprints/Unit/Unit` (`self.GetOwner`)))
  (bind _returnvalue_2 (`|GetDataTableRow` "/Game/DataTable/UnitDataTable.UnitDataTable" (`/Game/Blueprints/Unit/Unit.UnitKey` _asunit))
    (:`then`
      (bind (_unitname _unitclass _leveldatatable) (break `/Game/Blueprints/Struct/UnitData` _returnvalue_2))
      (bind _outrownames (`DataTableFunctionLibrary.GetDataTableRowNames` _leveldatatable))
      (for _array_element _outrownames
        (bind _returnvalue_3 (`|GetDataTableRow` _leveldatatable _array_element)
          (:`then`
            (`BlueprintMapLibrary.Map_Add` (`self.UnitLevelData`) (`KismetStringLibrary.Conv_StringToInt` (`KismetStringLibrary.Conv_NameToString` _array_element)) _returnvalue_3))))
      (if (`Actor.HasAuthority` (`self.GetOwner`))
        (set `self.Lv` 0)
        (`self.LevelUp`)
        (`/Engine/EditorBlueprintResources/StandardMacros.IsValid` _returnvalue
          (:`Is Valid`
            (`/Game/Blueprints/Component/HPMPComponent.FullRecovery` _returnvalue)))))))

(event `AddExp`
  (params (Exp :type "Float (double-precision)"))
  (set `self.Exp` (+ Exp (`self.Exp`)))
  (`self.LevelUp`))

(fn `GetAddParam`
  (params (Param :type "/Game/Blueprints/Enum/Param Enum" :default "NewEnumerator0"))
  (returns (Value :type "Float (double-precision)"))
  (bind (_value _returnvalue) (`BlueprintMapLibrary.Map_Find` (`self.UnitLevelData`) (`self.Lv`)))
  (bind (_exp _hp _mp _hpregen _mpregen _meleeattack _meleedefence _magicattack _magicdefence _attackspeed _attackrange _movementspeed) (break `/Game/Blueprints/Struct/UnitLevelData` _value))
  (if _returnvalue
    (return (select `/Game/Blueprints/Enum/Param` Param :`NewEnumerator0` _hp :`NewEnumerator1` _mp :`NewEnumerator2` _hpregen :`NewEnumerator3` _mpregen :`NewEnumerator4` _meleeattack :`NewEnumerator5` _meleedefence :`NewEnumerator6` _magicattack :`NewEnumerator7` _magicdefence :`NewEnumerator8` _attackspeed :`NewEnumerator9` _attackrange :`NewEnumerator10` _movementspeed))
    (else
      (return 0.0))))

(fn `GetMulParam`
  (params (Param :type "/Game/Blueprints/Enum/Param Enum" :default "NewEnumerator0"))
  (returns (Value :type "Float (double-precision)"))
  (return 1.0))

(fn `LevelUp`
  (bind (_value _returnvalue) (`BlueprintMapLibrary.Map_Find` (`self.UnitLevelData`) (+ (`self.Lv`) 1)))
  (if _returnvalue
    (if (>= (`self.Exp`) (`.Exp_13_19121752494E96A3BC216CB777530B13` (break `/Game/Blueprints/Struct/UnitLevelData` _value)))
      (`/Engine/EditorBlueprintResources/StandardMacros.IncrementInt` (`self.Lv`)
        (:`  `
          (`self.LevelUp`))))))