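; MyTargetPoint is a placeable target point actor marked with a unit key and a team.
; Its construction script shows the UnitKey on a text render component and colors the text yellow, blue or red to match the Team value.
; The event graph holds only disabled placeholder events, so it runs no gameplay logic of its own.
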(fn `UserConstructionScript`
  (`TextRenderComponent.K2_SetText` (`self.TextRender`) (`KismetTextLibrary.Conv_NameToText` (`self.UnitKey`)))
  (switch `/Game/Blueprints/Enum/Team` (`self.Team`)
    (:`NewEnumerator0`
      (`TextRenderComponent.SetTextRenderColor` (`self.TextRender`) (make `Color` 0 255 255)))
    (:`NewEnumerator1`
      (`TextRenderComponent.SetTextRenderColor` (`self.TextRender`) (make `Color` 255)))
    (:`NewEnumerator2`
      (`TextRenderComponent.SetTextRenderColor` (`self.TextRender`) (make `Color` 0 0 255)))))