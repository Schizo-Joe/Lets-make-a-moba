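; Base unit actor with team, stats, health, sight and an overhead or screen HUD, delegating to HPMP, Level, Sight and Event components.
; Tick shows or hides mesh and HUD by the local command unit's team vision, and syncs collision, attack animation speed and server-side walk speed.
; Damage makes idle or recalling AI retaliate; death awards exp and gold to the killer, stops AI and collision, and dispatches an event.
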(event `self.ReceiveBeginPlay`
  (bind _returnvalue (`GameplayStatics.GetPlayerController` 0))
  (`/Engine/EditorBlueprintResources/StandardMacros.IsValid` _returnvalue
    (:`Is Valid`
      (bind _returnvalue_2 (`|CreateWidget` "/Game/Blueprints/Widget/UnitHUD.UnitHUD_C" _returnvalue))
      (bind _output_get (set `self.HUD` _returnvalue_2))
      (`UserWidget.AddToViewport` _output_get 0))))

(event `self.ReceiveEndPlay`
  (params (EndPlayReason :type "EEndPlayReason Enum" :default "Destroyed"))
  (bind _hud (`self.HUD`))
  (`/Engine/EditorBlueprintResources/StandardMacros.IsValid` _hud
    (:`Is Valid`
      (`Widget.RemoveFromParent` _hud))))

(event `self.ReceiveTick`
  (params (DeltaSeconds :type "Float (single-precision)"))
  (bind _hud (`self.HUD`))
  (`|ExecutionSequence`
    (:`then_0`
      (bind _asmy_player_controller (cast `/Game/Blueprints/PlayerController/MyPlayerController` (`GameplayStatics.GetPlayerController` 0)))
      (bind _commandunit (`/Game/Blueprints/PlayerController/MyPlayerController.CommandUnit` _asmy_player_controller))
      (`/Engine/EditorBlueprintResources/StandardMacros.IsValid` _commandunit
        (:`Is Valid`
          (bind _vision (`self.GetVision` (`/Game/Blueprints/Unit/Unit.Team` _commandunit)))
          (`self.SetAppearance` _vision))))
    (:`then_1`
      (`/Engine/EditorBlueprintResources/StandardMacros.IsValid` _hud
        (:`Is Valid`
          (if (`Widget.IsVisible` _hud)
            (`/Game/Blueprints/Widget/UnitHUD.Update` _hud self)))))
    (:`then_2`
      (bind _value (`self.GetUnitParam` "NewEnumerator8"))
      (set `self.AttackSpeedForAnim` _value))
    (:`then_3`
      (`PrimitiveComponent.SetCollisionResponseToChannel` (`self.CapsuleComponent`) "ECC_Pawn" (select `bool` (`self.CollisionEnabled`) :`false` "ECR_Ignore" :`true` "ECR_Block" :!type "ECollisionResponse Enum")))
    (:`then_4`
      (`/Engine/EditorBlueprintResources/ActorMacros.Switch Has Authority`
        (:`Authority`
          (bind _value_2 (`self.GetUnitParam` "NewEnumerator10"))
          (set `CharacterMovementComponent.MaxWalkSpeed` _value_2 (`self.CharacterMovement`)))))))

(event `SetAppearance`
  (params (Vision :type "/Game/Blueprints/Enum/Vision Enum" :default "NewEnumerator0"))
  (bind _returnvalue (select `/Game/Blueprints/Enum/Vision` Vision :`NewEnumerator0` true :`NewEnumerator1` true))
  (`SceneComponent.SetVisibility` (`self.Mesh`) _returnvalue true)
  (bind _alive (`self.IsAlive`))
  (`Widget.SetVisibility` (`self.HUD`) (select `bool` (and _alive _returnvalue) :`false` "Hidden" :`true` "Visible" :!type "ESlateVisibility Enum")))

(event `Init`
  (params (UnitKey :type Name) (Team :type "/Game/Blueprints/Enum/Team Enum" :default "NewEnumerator0"))
  (set `self.UnitKey` UnitKey)
  (set `self.Team` Team)
  (`/Game/Blueprints/Component/EventComponent/EventComponent.Init` (`self.EventComponent`))
  (`/Game/Blueprints/Component/SightComponent.Init` (`self.SightComponent`)))

(event `/Game/Blueprints/Component/EventComponent/GetEventInterface.DispatchNormalEvent`
  (params (Event :type "/Game/Blueprints/Enum/NormalEvent Enum" :default "NewEnumerator0"))
  (`/Game/Blueprints/Component/EventComponent/GetEventInterface.DispatchNormalEvent` (`self.EventComponent`) Event))

(event `/Game/Blueprints/Component/EventComponent/GetEventInterface.DispatchByteEvent`
  (params (Event :type "/Game/Blueprints/Enum/ByteEvent Enum" :default "NewEnumerator0") (Byte :type Byte))
  (`/Game/Blueprints/Component/EventComponent/GetEventInterface.DispatchByteEvent` (`self.EventComponent`) Event Byte))

(event `self.ReceiveAnyDamage`
  (params (Damage :type "Float (single-precision)") (DamageType :type "DamageType Object Reference") (InstigatedBy :type "Controller Object Reference") (DamageCauser :type "Actor Object Reference"))
  (bind _alive (`self.IsAlive`))
  (if _alive
    (`/Game/Blueprints/Component/HPMPComponent.AddHP` (`self.HPMPComponent`) (- 0.0 Damage))
    (bind _alive_2 (`self.IsAlive`))
    (if _alive_2
      (bind _asunit_aicontroller (cast `/Game/Blueprints/Unit/UnitAIController` (`AIBlueprintHelperLibrary.GetAIController` self)))
      (switch `/Game/Blueprints/Enum/Command` (`/Game/Blueprints/Unit/UnitAIController.Command` _asunit_aicontroller)
        (:`NewEnumerator0`
          _)
        (:`NewEnumerator4`
          _))
      (bind _asunit (cast `/Game/Blueprints/Unit/Unit` DamageCauser))
      (`/Game/Blueprints/Unit/UnitAIController.SetCommand` _asunit_aicontroller "NewEnumerator2" (0.0 0.0 0.0) _asunit)
      (else
        (`|ExecutionSequence`
          (:`then_0`
            (bind _newparam (`self.GetExp`))
            (bind _newparam_2 (`self.GetGold`))
            (bind _asunit_2 (cast `/Game/Blueprints/Unit/Unit` DamageCauser))
            (`self.AddExpGold` _asunit_2 _newparam _newparam_2))
          (:`then_1`
            (bind _asunit_aicontroller_2 (cast `/Game/Blueprints/Unit/UnitAIController` (`AIBlueprintHelperLibrary.GetAIController` self)))
            (`/Game/Blueprints/Unit/UnitAIController.SetCommand` _asunit_aicontroller_2 "NewEnumerator0" (0.0 0.0 0.0) null)
            (`BrainComponent.StopLogic` (`AIController.BrainComponent` _asunit_aicontroller_2) "")
            (set `self.Anim` "NewEnumerator3")
            (set `self.CollisionEnabled` false)
            (`/Game/Blueprints/Component/EventComponent/GetEventInterface.DispatchNormalEvent` "NewEnumerator0")))))))

(event `AddExpGold`
  (params (Exp :type "Float (double-precision)") (Gold :type Integer))
  (bind _returnvalue (`self.GetComponentByClass` "/Game/Blueprints/Component/InventoryComponent.InventoryComponent_C"))
  (`/Game/Blueprints/Component/LevelComponent.AddExp` (`self.LevelComponent`) Exp)
  (`/Engine/EditorBlueprintResources/StandardMacros.IsValid` _returnvalue
    (:`Is Valid`
      (`/Game/Blueprints/Component/InventoryComponent.AddGold` _returnvalue Gold))))

(fn `GetByteEventDispatcher`
  (params (Event :type "/Game/Blueprints/Enum/ByteEvent Enum" :default "NewEnumerator0"))
  (returns (Wrapper :type "/Game/Blueprints/Component/EventComponent/ByteEventDispatcherWrapper Object Reference"))
  (bind _wrapper (`/Game/Blueprints/Component/EventComponent/GetEventInterface.GetByteEventDispatcher` (`self.EventComponent`) Event))
  (return _wrapper))

(fn `GetExp`
  (returns (NewParam :type "Float (double-precision)"))
  (return 0.0))

(fn `GetGold`
  (returns (NewParam :type Integer))
  (return 0))

(fn `GetNormalEventDispatcher`
  (params (Event :type "/Game/Blueprints/Enum/NormalEvent Enum" :default "NewEnumerator0"))
  (returns (Wrapper :type "/Game/Blueprints/Component/EventComponent/NormalEventDispatcherWrapper Object Reference"))
  (bind _wrapper (`/Game/Blueprints/Component/EventComponent/GetEventInterface.GetNormalEventDispatcher` (`self.EventComponent`) Event))
  (return _wrapper))

(fn `GetUnitParam`
  (params (Param :type "/Game/Blueprints/Enum/Param Enum" :default "NewEnumerator0"))
  (returns (Value :type "Float (double-precision)"))
  (bind _value (`/Game/Blueprints/Component/GetParamInterface.GetAddParam` (`self.LevelComponent`) Param))
  (return _value))

(fn `GetVision`
  (params (Team :type "/Game/Blueprints/Enum/Team Enum" :default "NewEnumerator0"))
  (returns (Vision :type "/Game/Blueprints/Enum/Vision Enum"))
  (bind _visible (`/Game/Blueprints/Component/SightComponent.GetSight` (`self.SightComponent`) Team))
  (return (select `bool` (and _visible (`self.UnitVisible`)) :`false` "NewEnumerator2" :`true` "NewEnumerator0" :!type "/Game/Blueprints/Enum/Vision Enum")))

(fn `IsAlive`
  (returns (Alive :type Boolean))
  (bind _alive (`/Game/Blueprints/Component/HPMPComponent.IsAlive` (`self.HPMPComponent`)))
  (return _alive))

(fn `OnRep_UnitKey`
  (`/Game/Blueprints/Component/LevelComponent.Init` (`self.LevelComponent`)))

(fn `UserConstructionScript`)