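; Inventory component that manages a unit's gold and item slots, storing data table row names with "None" marking empty slots.
; Buy and Sell check the item's table row, then update gold and slots.
; Consume spawns the row's consume-item actor, applies it to the owning Unit, destroys it and clears the slot.
; GetAddParam and GetMulParam combine held items' additive and multiplicative bonuses for a requested stat.
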(event `AddGold`
  (params (Gold :type Integer))
  (set `self.Gold` (+ Gold (`self.Gold`))))

(event `AddItem`
  (params (ItemKey :type Name))
  (bind (_found _index) (`self.GetEmptySlot`))
  (if _found
    (`|GetDataTableRow` "/Game/DataTable/ItemDataTable.ItemDataTable" ItemKey
      (:`then`
        (`KismetArrayLibrary.Array_Set` (`self.ItemKeys`) _index ItemKey)))))

(event `Consume`
  (params (Index :type Integer))
  (bind _output (`|GetArrayItem` (`self.ItemKeys`) Index))
  (bind _returnvalue (`|GetDataTableRow` "/Game/DataTable/ItemDataTable.ItemDataTable" _output)
    (:`then`
      (bind (_itemname _icontexture _description _buyprice _sellprice _consumeitemclass) (break `/Game/Blueprints/Struct/ItemData` _returnvalue))
      (if (`KismetSystemLibrary.IsValidClass` _consumeitemclass)
        (bind _returnvalue_2 (`|SpawnActorFromClass` _consumeitemclass (`KismetMathLibrary.MakeTransform` (0.0 0.0 0.0)) "AlwaysSpawn" "OverrideRootScale" null null))
        (bind _asunit (cast `/Game/Blueprints/Unit/Unit` (`self.GetOwner`)))
        (`/Game/Blueprints/Item/ConsumeItem.Consume` _returnvalue_2 _asunit _output)
        (`Actor.K2_DestroyActor` _returnvalue_2)
        (`self.RemoveItem` Index)))))

(event `RemoveItem`
  (params (Index :type Integer))
  (`KismetArrayLibrary.Array_Set` (`self.ItemKeys`) Index))

(event `Sell`
  (params (Index :type Integer))
  (bind _itemkey (`self.GetItem` Index))
  (if (!= _itemkey "None")
    (bind _returnvalue (`|GetDataTableRow` "/Game/DataTable/ItemDataTable.ItemDataTable" _itemkey)
      (:`then`
        (`self.RemoveItem` Index)
        (`self.AddGold` (`.SellPrice_14_14AC247C4BCF2A5A020C4AA922227E8E` (break `/Game/Blueprints/Struct/ItemData` _returnvalue)))))))

(event `Buy`
  (params (ItemKey :type Name))
  (bind _found (`self.GetEmptySlot`))
  (if _found
    (bind _returnvalue (`|GetDataTableRow` "/Game/DataTable/ItemDataTable.ItemDataTable" ItemKey)
      (:`then`
        (bind (_itemname _icontexture _description _buyprice) (break `/Game/Blueprints/Struct/ItemData` _returnvalue))
        (if (>= (`self.Gold`) _buyprice)
          (`self.AddGold` (- 0 _buyprice))
          (`self.AddItem` ItemKey))))))

(fn `GetAddParam`
  (params (Param :type "/Game/Blueprints/Enum/Param Enum" :default "NewEnumerator0"))
  (returns (Value :type "Float (double-precision)"))
  (locals (Sum :type "Float (double-precision)"))
  (for _array_element (`self.ItemKeys`)
    (if (!= _array_element "None")
      (bind _returnvalue (`|GetDataTableRow` "/Game/DataTable/ItemDataTable.ItemDataTable" _array_element)
        (:`then`
          (bind (_itemname _icontexture _description _buyprice _sellprice _consumeitemclass _addhp _addmp _addhpregen _addmpregen _addmeleeattack _addmeleedefence _addmagicattack _addmagicdefence _addattackspeed _addattackrange _addmovementspeed) (break `/Game/Blueprints/Struct/ItemData` _returnvalue))
          (set `local.Sum` (+ (`local.Sum`) (select `/Game/Blueprints/Enum/Param` Param :`NewEnumerator0` _addhp :`NewEnumerator1` _addmp :`NewEnumerator2` _addhpregen :`NewEnumerator3` _addmpregen :`NewEnumerator4` _addmeleeattack :`NewEnumerator5` _addmeleedefence :`NewEnumerator6` _addmagicattack :`NewEnumerator7` _addmagicdefence :`NewEnumerator8` _addattackspeed :`NewEnumerator9` _addattackrange :`NewEnumerator10` _addmovementspeed)))))))
  (return (`local.Sum`)))

(fn `GetEmptySlot`
  (returns (Found :type Boolean) (Index :type Integer))
  (for (_array_element _array_index) (`self.ItemKeys`)
    (if (== _array_element "None")
      (return true _array_index)))
  (return false 0))

(fn `GetItem`
  (params (Index :type Integer))
  (returns (ItemKey :type Name))
  (return (`|GetArrayItem` (`self.ItemKeys`) Index)))

(fn `GetMaxItemNum`
  (returns (MaxNum :type Integer))
  (return (`KismetArrayLibrary.Array_Length` (`self.ItemKeys`))))

(fn `GetMulParam`
  (params (Param :type "/Game/Blueprints/Enum/Param Enum" :default "NewEnumerator0"))
  (returns (Value :type "Float (double-precision)"))
  (locals (Sum :type "Float (double-precision)" :default 1.0))
  (for _array_element (`self.ItemKeys`)
    (if (!= _array_element "None")
      (bind _returnvalue (`|GetDataTableRow` "/Game/DataTable/ItemDataTable.ItemDataTable" _array_element)
        (:`then`
          (bind (_itemname _icontexture _description _buyprice _sellprice _consumeitemclass _addhp _addmp _addhpregen _addmpregen _addmeleeattack _addmeleedefence _addmagicattack _addmagicdefence _addattackspeed _addattackrange _addmovementspeed _mulhp _mulmp _mulhpregen _mulmpregen _mulmeleeattack _mulmeleedefence _mulmagicattack _mulmagicdefence _mulattackspeed _mulattackrange _mulmovementspeed) (break `/Game/Blueprints/Struct/ItemData` _returnvalue))
          (set `local.Sum` (* (`local.Sum`) (select `/Game/Blueprints/Enum/Param` Param :`NewEnumerator0` _mulhp :`NewEnumerator1` _mulmp :`NewEnumerator2` _mulhpregen :`NewEnumerator3` _mulmpregen :`NewEnumerator4` _mulmeleeattack :`NewEnumerator5` _mulmeleedefence :`NewEnumerator6` _mulmagicattack :`NewEnumerator7` _mulmagicdefence :`NewEnumerator8` _mulattackspeed :`NewEnumerator9` _mulattackrange :`NewEnumerator10` _mulmovementspeed)))))))
  (return (`local.Sum`)))