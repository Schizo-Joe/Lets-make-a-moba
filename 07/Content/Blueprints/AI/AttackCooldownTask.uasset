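; Behavior tree task that holds an AI-controlled Unit through an attack cooldown.
; On its Tick event it gets the controlled Unit from the UnitAIController, reads one unit parameter and looks up the unit's row in UnitDataTable.
; It delays for that parameter scaled by one minus the row's AttackingRate, then finishes with success.
; A failed cast stops the flow, and only the row-found branch reaches the finish.
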(event `self.ReceiveTick`
  (params (OwnerActor :type "Actor Object Reference") (DeltaSeconds :type "Float (single-precision)"))
  (bind _asunit_aicontroller (cast `/Game/Blueprints/Unit/UnitAIController` OwnerActor))
  (bind _asunit (cast `/Game/Blueprints/Unit/Unit` (`Controller.K2_GetPawn` _asunit_aicontroller)))
  (bind _value (`/Game/Blueprints/Unit/Unit.GetUnitParam` _asunit "NewEnumerator8"))
  (bind _returnvalue (`|GetDataTableRow` "/Game/DataTable/UnitDataTable.UnitDataTable" (`/Game/Blueprints/Unit/Unit.UnitKey` _asunit))
    (:`then`
      (`KismetSystemLibrary.Delay` (* _value (- 1.0 (`.AttackingRate_11_84A0032A4DBE8C91B013DA84621F42E3` (break `/Game/Blueprints/Struct/UnitData` _returnvalue)))))
      (`self.FinishExecute` true))))