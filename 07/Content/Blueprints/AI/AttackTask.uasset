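; Behavior Tree task that runs an AI-controlled unit's attack on the blackboard's target unit, currently only a debug print.
; On tick it yaws the unit toward the target, then waits for the AttackingRate from the unit data table scaled by a unit parameter.
; After the delay it checks distance against another unit parameter, printing "Attack" and succeeding when in range, otherwise failing.
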(event `self.ReceiveTick`
  (params (OwnerActor :type "Actor Object Reference") (DeltaSeconds :type "Float (single-precision)"))
  (bind _controlledunit (`self.ControlledUnit`))
  (bind _controlledunit_2 (`self.ControlledUnit`))
  (bind _asunit_aicontroller (cast `/Game/Blueprints/Unit/UnitAIController` OwnerActor))
  (bind _asunit (cast `/Game/Blueprints/Unit/Unit` (`Controller.K2_GetPawn` _asunit_aicontroller)))
  (set `self.ControlledUnit` _asunit)
  (bind _asunit_2 (cast `/Game/Blueprints/Unit/Unit` (`BTFunctionLibrary.GetBlackboardValueAsObject` (`self.TargetUnitKey`))))
  (set `self.TargetUnit` _asunit_2)
  (`self.SetControlledUnitRotation`
    (:`Rotate`
      (bind _value (`/Game/Blueprints/Unit/Unit.GetUnitParam` _controlledunit "NewEnumerator8"))
      (bind _returnvalue (`|GetDataTableRow` "/Game/DataTable/UnitDataTable.UnitDataTable" (`/Game/Blueprints/Unit/Unit.UnitKey` _controlledunit))
        (:`then`
          (`KismetSystemLibrary.Delay` (* (`.AttackingRate_11_84A0032A4DBE8C91B013DA84621F42E3` (break `/Game/Blueprints/Struct/UnitData` _returnvalue)) _value))
          (bind _distance (`/Game/Blueprints/Library/MyLibrary.GetUnitDistance` _controlledunit_2 (`self.TargetUnit`)))
          (bind _value_2 (`/Game/Blueprints/Unit/Unit.GetUnitParam` _controlledunit_2 "NewEnumerator9"))
          (if (<= _distance _value_2)
            (`KismetSystemLibrary.PrintString` "Attack")
            (`self.FinishExecute` true)
            (else
              (`self.FinishExecute` false))))))))