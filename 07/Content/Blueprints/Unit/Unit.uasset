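; Base Character Blueprint for a networked, team-based game unit, delegating events, sight, health and stat parameters to components.
; Init sets UnitKey and Team and starts the event and sight components, while UnitKey replication initializes LevelComponent.
; Each tick it shows or hides the mesh and its HUD widget by the local CommandUnit team's vision, with the HUD also requiring life.
; Tick also refreshes attack animation speed and, on the server, walk speed from LevelComponent.
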(event `self.ReceiveBeginPlay`
  (bind _returnvalue (`GameplayStatics.GetPlayerController` 0))
  (`/Engine/EditorBlueprintResources/StandardMacros.IsValid` _returnvalue
    (:`Is Valid`
      (bind _returnvalue_2 (`|CreateWidget` "/Game/Blueprints/Widget/UnitHUD.UnitHUD_C" _returnvalue))
      (bind _output_get (set `self.HUD` _returnvalue_2))
      (`UserWidget.AddToViewport` _output_get 0))))

(event `self.ReceiveEndPlay`
  (params (EndPlayReason :type "EEndPlayReason Enum" :default "Destroyed"))
  (bind _hud (`self.HUD`))
  (`/Engine/EditorBlueprintResources/StandardMacros.IsValid` _hud
    (:`Is Valid`
      (`Widget.RemoveFromParent` _hud))))

(event `self.ReceiveTick`
  (params (DeltaSeconds :type "Float (single-precision)"))
  (bind _hud (`self.HUD`))
  (`|ExecutionSequence`
    (:`then_0`
      (bind _asmy_player_controller (cast `/Game/Blueprints/PlayerController/MyPlayerController` (`GameplayStatics.GetPlayerController` 0)))
      (bind _commandunit (`/Game/Blueprints/PlayerController/MyPlayerController.CommandUnit` _asmy_player_controller))
      (`/Engine/EditorBlueprintResources/StandardMacros.IsValid` _commandunit
        (:`Is Valid`
          (bind _vision (`self.GetVision` (`/Game/Blueprints/Unit/Unit.Team` _commandunit)))
          (`self.SetAppearance` _vision))))
    (:`then_1`
      (`/Engine/EditorBlueprintResources/StandardMacros.IsValid` _hud
        (:`Is Valid`
          (if (`Widget.IsVisible` _hud)
            (`/Game/Blueprints/Widget/UnitHUD.Update` _hud self)))))
    (:`then_2`
      (bind _value (`self.GetUnitParam` "NewEnumerator8"))
      (set `self.AttackSpeedForAnim` _value))
    (:`then_3`
      (`/Engine/EditorBlueprintResources/ActorMacros.Switch Has Authority`
        (:`Authority`
          (bind _value_2 (`self.GetUnitParam` "NewEnumerator10"))
          (set `CharacterMovementComponent.MaxWalkSpeed` _value_2 (`self.CharacterMovement`)))))))

(event `SetAppearance`
  (params (Vision :type "/Game/Blueprints/Enum/Vision Enum" :default "NewEnumerator0"))
  (bind _returnvalue (select `/Game/Blueprints/Enum/Vision` Vision :`NewEnumerator0` true :`NewEnumerator1` true))
  (`SceneComponent.SetVisibility` (`self.Mesh`) _returnvalue true)
  (bind _alive (`self.IsAlive`))
  (`Widget.SetVisibility` (`self.HUD`) (select `bool` (and _alive _returnvalue) :`false` "Hidden" :`true` "Visible" :!type "ESlateVisibility Enum")))

(event `Init`
  (params (UnitKey :type Name) (Team :type "/Game/Blueprints/Enum/Team Enum" :default "NewEnumerator0"))
  (set `self.UnitKey` UnitKey)
  (set `self.Team` Team)
  (`/Game/Blueprints/Component/EventComponent/EventComponent.Init` (`self.EventComponent`))
  (`/Game/Blueprints/Component/SightComponent.Init` (`self.SightComponent`)))

(event `/Game/Blueprints/Component/EventComponent/GetEventInterface.DispatchNormalEvent`
  (params (Event :type "/Game/Blueprints/Enum/NormalEvent Enum" :default "NewEnumerator0"))
  (`/Game/Blueprints/Component/EventComponent/GetEventInterface.DispatchNormalEvent` (`self.EventComponent`) Event))

(event `/Game/Blueprints/Component/EventComponent/GetEventInterface.DispatchByteEvent`
  (params (Event :type "/Game/Blueprints/Enum/ByteEvent Enum" :default "NewEnumerator0") (Byte :type Byte))
  (`/Game/Blueprints/Component/EventComponent/GetEventInterface.DispatchByteEvent` (`self.EventComponent`) Event Byte))

(fn `GetByteEventDispatcher`
  (params (Event :type "/Game/Blueprints/Enum/ByteEvent Enum" :default "NewEnumerator0"))
  (returns (Wrapper :type "/Game/Blueprints/Component/EventComponent/ByteEventDispatcherWrapper Object Reference"))
  (bind _wrapper (`/Game/Blueprints/Component/EventComponent/GetEventInterface.GetByteEventDispatcher` (`self.EventComponent`) Event))
  (return _wrapper))

(fn `GetNormalEventDispatcher`
  (params (Event :type "/Game/Blueprints/Enum/NormalEvent Enum" :default "NewEnumerator0"))
  (returns (Wrapper :type "/Game/Blueprints/Component/EventComponent/NormalEventDispatcherWrapper Object Reference"))
  (bind _wrapper (`/Game/Blueprints/Component/EventComponent/GetEventInterface.GetNormalEventDispatcher` (`self.EventComponent`) Event))
  (return _wrapper))

(fn `GetUnitParam`
  (params (Param :type "/Game/Blueprints/Enum/Param Enum" :default "NewEnumerator0"))
  (returns (Value :type "Float (double-precision)"))
  (bind _value (`/Game/Blueprints/Component/GetParamInterface.GetAddParam` (`self.LevelComponent`) Param))
  (return _value))

(fn `GetVision`
  (params (Team :type "/Game/Blueprints/Enum/Team Enum" :default "NewEnumerator0"))
  (returns (Vision :type "/Game/Blueprints/Enum/Vision Enum"))
  (bind _visible (`/Game/Blueprints/Component/SightComponent.GetSight` (`self.SightComponent`) Team))
  (return (select `bool` (and _visible (`self.UnitVisible`)) :`false` "NewEnumerator2" :`true` "NewEnumerator0" :!type "/Game/Blueprints/Enum/Vision Enum")))

(fn `IsAlive`
  (returns (Alive :type Boolean))
  (bind _alive (`/Game/Blueprints/Component/HPMPComponent.IsAlive` (`self.HPMPComponent`)))
  (return _alive))

(fn `OnRep_UnitKey`
  (`/Game/Blueprints/Component/LevelComponent.Init` (`self.LevelComponent`)))

(fn `UserConstructionScript`)