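; Unit is the Blueprint for a team unit that moves by AI, identified by a unit key and team set in Init.
; BeginPlay creates a UnitHUD widget for player controller 0, Tick updates it with the unit, and EndPlay removes it.
; Move switches the Anim enum around an AIMoveTo, resetting it only on success.
; An EventComponent handles normal and byte event dispatching through pass-through functions on the unit.
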(event `self.ReceiveBeginPlay`
  (bind _returnvalue (`GameplayStatics.GetPlayerController` 0))
  (`/Engine/EditorBlueprintResources/StandardMacros.IsValid` _returnvalue
    (:`Is Valid`
      (bind _returnvalue_2 (`|CreateWidget` "/Game/Blueprints/Widget/UnitHUD.UnitHUD_C" _returnvalue))
      (bind _output_get (set `self.HUD` _returnvalue_2))
      (`UserWidget.AddToViewport` _output_get 0))))

(event `self.ReceiveEndPlay`
  (params (EndPlayReason :type "EEndPlayReason Enum" :default "Destroyed"))
  (bind _hud (`self.HUD`))
  (`/Engine/EditorBlueprintResources/StandardMacros.IsValid` _hud
    (:`Is Valid`
      (`Widget.RemoveFromParent` _hud))))

(event `self.ReceiveTick`
  (params (DeltaSeconds :type "Float (single-precision)"))
  (bind _hud (`self.HUD`))
  (`/Engine/EditorBlueprintResources/StandardMacros.IsValid` _hud
    (:`Is Valid`
      (`/Game/Blueprints/Widget/UnitHUD.Update` _hud self))))

(event `Init`
  (params (UnitKey :type Name) (Team :type "/Game/Blueprints/Enum/Team Enum" :default "NewEnumerator0"))
  (set `self.UnitKey` UnitKey)
  (set `self.Team` Team)
  (`/Game/Blueprints/Component/EventComponent/EventComponent.Init` (`self.EventComponent`)))

(event `/Game/Blueprints/Component/EventComponent/GetEventInterface.DispatchNormalEvent`
  (params (Event :type "/Game/Blueprints/Enum/NormalEvent Enum" :default "NewEnumerator0"))
  (`/Game/Blueprints/Component/EventComponent/GetEventInterface.DispatchNormalEvent` (`self.EventComponent`) Event))

(event `/Game/Blueprints/Component/EventComponent/GetEventInterface.DispatchByteEvent`
  (params (Event :type "/Game/Blueprints/Enum/ByteEvent Enum" :default "NewEnumerator0") (Byte :type Byte))
  (`/Game/Blueprints/Component/EventComponent/GetEventInterface.DispatchByteEvent` (`self.EventComponent`) Event Byte))

(event `Move`
  (params (Destination :type "Vector Structure"))
  (set `self.Anim` "NewEnumerator1")
  (`|AIMoveTo` self Destination
    (:`OnSuccess`
      (set `self.Anim` "NewEnumerator0"))))

(fn `GetByteEventDispatcher`
  (params (Event :type "/Game/Blueprints/Enum/ByteEvent Enum" :default "NewEnumerator0"))
  (returns (Wrapper :type "/Game/Blueprints/Component/EventComponent/ByteEventDispatcherWrapper Object Reference"))
  (bind _wrapper (`/Game/Blueprints/Component/EventComponent/GetEventInterface.GetByteEventDispatcher` (`self.EventComponent`) Event))
  (return _wrapper))

(fn `GetNormalEventDispatcher`
  (params (Event :type "/Game/Blueprints/Enum/NormalEvent Enum" :default "NewEnumerator0"))
  (returns (Wrapper :type "/Game/Blueprints/Component/EventComponent/NormalEventDispatcherWrapper Object Reference"))
  (bind _wrapper (`/Game/Blueprints/Component/EventComponent/GetEventInterface.GetNormalEventDispatcher` (`self.EventComponent`) Event))
  (return _wrapper))

(fn `UserConstructionScript`)